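; Test planet actor that orbits a center point, intended to become the black hole's center.
; On BeginPlay it moves the actor to Center and puts the Sphere back at the spawn transform, making the actor origin the orbit pivot.
; It then sets a random starting yaw, so the planet's orbital phase varies.
; Tick increases yaw at a constant rate scaled by delta time, swinging the offset Sphere around Center.
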(event `self.ReceiveBeginPlay`
  (bind (_initiallocation_location _initiallocation_rotation) (`KismetMathLibrary.BreakTransform` (`self.InitialLocation`)))
  ; 여기서 돌기 시작
  (set `self.InitialLocation` (`self.GetTransform`))
  (`self.K2_SetActorLocationAndRotation` (`self.Center`))
  (`SceneComponent.K2_SetWorldLocationAndRotation` (`self.Sphere`) _initiallocation_location _initiallocation_rotation false false)
  (`self.K2_SetActorRotation` (`KismetMathLibrary.MakeRotator` 0.0 0.0 (`KismetMathLibrary.RandomFloatInRange` 0.0 360.0))))

(event `self.ReceiveTick`
  (params (DeltaSeconds :type "Float (single-precision)"))
  (bind (_returnvalue_roll _returnvalue_pitch _returnvalue_yaw) (`KismetMathLibrary.BreakRotator` (`self.K2_GetActorRotation`)))
  (`self.K2_SetActorRotation` (`KismetMathLibrary.MakeRotator` 0.0 0.0 (+ (* DeltaSeconds 100.0) _returnvalue_yaw))))

(fn `UserConstructionScript`)