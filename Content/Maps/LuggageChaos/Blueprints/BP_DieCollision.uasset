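; BP_DieCollision is a kill volume in the LuggageChaos map that handles characters and luggage falling into it.
; It caches the LuggageChaos game state on BeginPlay.
; On overlap, a player-controlled BaseCharacter is reported to the game state's OnPlayerDeath, while Luggage is passed to a luggage manager reference to be reset.
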(event `self.ReceiveBeginPlay`
  (bind _asluggage_chaos_game_state (cast `LuggageChaosGameState` (`GameplayStatics.GetGameState`)))
  (bind _output_get (set `self.gs` _asluggage_chaos_game_state)))

(event `self.ReceiveActorBeginOverlap`
  (params (OtherActor :type "Actor Object Reference"))
  (bind _asbase_character (cast `BaseCharacter` OtherActor)
    (:`then`
      (bind _asplayer_controller (cast `PlayerController` (`Pawn.GetController` _asbase_character)))
      (`LuggageChaosGameState.OnPlayerDeath` (stale `self.ReceiveBeginPlay` _output_get) _asplayer_controller))
    (:`CastFailed`
      (bind _asluggage (cast `Luggage` OtherActor))
      (`LuggageManager.ResetLuggage` (`self.lugManager`) _asluggage))))

(fn `UserConstructionScript`)