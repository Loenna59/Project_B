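; Black hole actor that pulls every BoxAsset actor in the level toward itself.
; Each Tick it gathers all BoxAsset actors and overwrites each Box's physics velocity with a fixed-speed vector aimed at its 1r component, so the pull ignores distance and prior momentum.
; Comments label this phase 1 and note a possible player state variable for later.
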(event `self.ReceiveTick`
  (params (DeltaSeconds :type "Float (single-precision)"))
  ; 1페이즈
  ;; 나중에 플레이어 상태 변수 추가?
  (bind _outactors (`GameplayStatics.GetAllActorsOfClass` "/Script/Project_B.BoxAsset"))
  (for _array_element _outactors
    (`PrimitiveComponent.SetPhysicsLinearVelocity` (`BoxAsset.Box` _array_element) (* (`KismetMathLibrary.GetForwardVector` (`KismetMathLibrary.FindLookAtRotation` (`SceneComponent.K2_GetComponentLocation` (`BoxAsset.Box` _array_element)) (`SceneComponent.K2_GetComponentLocation` (`self.1r`)))) 200.0) false "None")))

(fn `UserConstructionScript`)